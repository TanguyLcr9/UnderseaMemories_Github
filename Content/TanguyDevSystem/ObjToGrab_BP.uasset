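; Grabbable object that the third-person character picks up by clicking while inside its trigger collider.
; The trigger swaps the cylinder to a highlight material and sets the player's hint text, clearing both on exit.
; Tick polls the player's click state, then passes the object's Type to the character and destroys the actor.
; Type 10 requires the player to have a tool (gloves) and shows French safety hints accordingly.
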(event OnComponentBeginOverlap(TrigerCollider)
  (params (OverlappedComponent :type Primitive%20Component%20Object%20Reference) (OtherActor :type Actor%20Object%20Reference) (OtherComp :type Primitive%20Component%20Object%20Reference) (OtherBodyIndex :type Integer) (bFromSweep :type Boolean) (SweepResult :type Hit%20Result%20Structure%20%28by%20ref%29))
  (bind _asthird_person_character (Utilities|Casting|CastToThirdPersonCharacter OtherActor))
  (if (== (Variables|Default|GetType) 10)
    (if (Variables|/Game/ThirdPersonBP/Blueprints/ThirdPersonCharacter.ThirdPersonCharacter_C|GetHasTool _asthird_person_character)
      (Variables|/Game/ThirdPersonBP/Blueprints/ThirdPersonCharacter.ThirdPersonCharacter_C|SetTextToDisplay _asthird_person_character "C'est bon je vais pouvoir me servir de mes gants pour manipuler le mécanisme en toute sécurité")
      (else
        (Variables|/Game/ThirdPersonBP/Blueprints/ThirdPersonCharacter.ThirdPersonCharacter_C|SetTextToDisplay _asthird_person_character "Ca m'a l'air dangeureux de toucher à ça tout de suite. Mieux vaux trouver un moyen plus sécurisant")))
    (else
      (Variables|/Game/ThirdPersonBP/Blueprints/ThirdPersonCharacter.ThirdPersonCharacter_C|SetTextToDisplay _asthird_person_character (Variables|Default|GetMyText))))
  (Variables|Default|SetPlayerIsOverlapping true)
  (Rendering|Material|SetMaterial (Variables|Default|GetCylinder) 0 "/Game/TanguyDevSystem/Materials/Over_Mat_Inst.Over_Mat_Inst"))

(event OnComponentEndOverlap(TrigerCollider)
  (params (OverlappedComponent :type Primitive%20Component%20Object%20Reference) (OtherActor :type Actor%20Object%20Reference) (OtherComp :type Primitive%20Component%20Object%20Reference) (OtherBodyIndex :type Integer))
  (bind _asthird_person_character (Utilities|Casting|CastToThirdPersonCharacter OtherActor))
  (Variables|/Game/ThirdPersonBP/Blueprints/ThirdPersonCharacter.ThirdPersonCharacter_C|SetTextToDisplay _asthird_person_character "")
  (Variables|Default|SetPlayerIsOverlapping false)
  (Rendering|Material|SetMaterial (Variables|Default|GetCylinder) 0 "/Game/ThirdPerson/Meshes/RampMaterial.RampMaterial"))

(event EventBeginPlay)

(event Collision|EventActorBeginOverlap
  (params (OtherActor :type Actor%20Object%20Reference)))

(event EventTick
  (params (DeltaSeconds :type Float%20%28single-precision%29))
  (if (Variables|Default|GetPlayerIsOverlapping)
    (bind _asthird_person_character (Utilities|Casting|CastToThirdPersonCharacter (Game|Player|GetPlayerPawn 0)))
    (if (Variables|/Game/ThirdPersonBP/Blueprints/ThirdPersonCharacter.ThirdPersonCharacter_C|GetClicking _asthird_person_character)
      (if (== (Variables|Default|GetType) 10)
        (if (Variables|/Game/ThirdPersonBP/Blueprints/ThirdPersonCharacter.ThirdPersonCharacter_C|GetHasTool _asthird_person_character)
          (if (not (Variables|Default|GetisAttachToPlayer)) :!label _label
            (Variables|Default|SetisAttachToPlayer true)
            (Variables|/Game/ThirdPersonBP/Blueprints/ThirdPersonCharacter.ThirdPersonCharacter_C|SetObjectType _asthird_person_character (Variables|Default|GetType))
            (Actor|DestroyActor)))
        (else
          (goto _label))))))

(fn ConstructionScript)