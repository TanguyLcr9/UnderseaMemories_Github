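; A dialogue trigger box that shows a line of text when the third-person character first enters it.
; On collision overlap it writes MyText into the character's TextToDisplay, then clears it after a TimeDisplayText delay.
; The TextAlreadyDisplay flag is never reset, so each box fires only once.
; The MyTask deactivation event is empty, and a second clearing path through the player pawn is unconnected.
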(event OnComponentBeginOverlap(CollisionComponent)
  (params (OverlappedComponent :type Primitive%20Component%20Object%20Reference) (OtherActor :type Actor%20Object%20Reference) (OtherComp :type Primitive%20Component%20Object%20Reference) (OtherBodyIndex :type Integer) (bFromSweep :type Boolean) (SweepResult :type Hit%20Result%20Structure%20%28by%20ref%29))
  (if (not (Variables|Default|GetTextAlreadyDisplay))
    (bind _asthird_person_character (Utilities|Casting|CastToThirdPersonCharacter OtherActor))
    (Variables|/Game/ThirdPersonBP/Blueprints/ThirdPersonCharacter.ThirdPersonCharacter_C|SetTextToDisplay _asthird_person_character (Variables|Default|GetMyText))
    (Variables|Default|SetTextAlreadyDisplay true)
    (Utilities|FlowControl|Delay (Variables|Default|GetTimeDisplayText))
    (Variables|/Game/ThirdPersonBP/Blueprints/ThirdPersonCharacter.ThirdPersonCharacter_C|SetTextToDisplay _asthird_person_character "")))

(event OnComponentDeactivated(MyTask)
  (params (Component :type Actor%20Component%20Object%20Reference)))

(event EventBeginPlay)

(event Collision|EventActorBeginOverlap
  (params (OtherActor :type Actor%20Object%20Reference)))

(event EventTick
  (params (DeltaSeconds :type Float%20%28single-precision%29)))

(fn ConstructionScript)