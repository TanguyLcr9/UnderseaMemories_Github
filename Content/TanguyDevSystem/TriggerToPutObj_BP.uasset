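; Trigger actor where the player places a carried object of a required type to swing a door open.
; While the player overlaps, Tick checks the character's ObjectType and shows prompt text on a match.
; A first click reveals the hidden object with collision, changes the base material, clears the carried type and plays a timeline rotating DoorRoot in yaw.
; Leaving clears the prompt and restores the base material cached at BeginPlay.
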(event OnComponentBeginOverlap(Trigger)
  (params (OverlappedComponent :type Primitive%20Component%20Object%20Reference) (OtherActor :type Actor%20Object%20Reference) (OtherComp :type Primitive%20Component%20Object%20Reference) (OtherBodyIndex :type Integer) (bFromSweep :type Boolean) (SweepResult :type Hit%20Result%20Structure%20%28by%20ref%29))
  ;[1 1 1] Comment
  (bind _asthird_person_character (Utilities|Casting|CastToThirdPersonCharacter OtherActor))
  (Variables|Default|SetPlayerIsOverlapping true)
  (if (== (Variables|/Game/ThirdPersonBP/Blueprints/ThirdPersonCharacter.ThirdPersonCharacter_C|GetObjectType _asthird_person_character) (Variables|Default|GetObjectTypeRequirement))
    (if (not (Variables|Default|GetObjetPut))
      (Rendering|Material|SetMaterial (Variables|Default|GetObjectBase) 0 (Variables|Default|GetMaterial)))))

(event OnComponentEndOverlap(Trigger)
  (params (OverlappedComponent :type Primitive%20Component%20Object%20Reference) (OtherActor :type Actor%20Object%20Reference) (OtherComp :type Primitive%20Component%20Object%20Reference) (OtherBodyIndex :type Integer))
  ;[1 1 1] Comment
  (bind _asthird_person_character (Utilities|Casting|CastToThirdPersonCharacter OtherActor))
  (Variables|Default|SetPlayerIsOverlapping false)
  (Variables|/Game/ThirdPersonBP/Blueprints/ThirdPersonCharacter.ThirdPersonCharacter_C|SetTextToDisplay _asthird_person_character "")
  (Rendering|Material|SetMaterial (Variables|Default|GetObjectBase) 0 (Variables|Default|GetMaterial)))

(event EventBeginPlay
  (bind _objecttodisplay (Variables|Default|GetObjectToDisplay))
  (Rendering|SetVisibility _objecttodisplay false false)
  (Collision|SetCollisionEnabled _objecttodisplay "NoCollision")
  (Variables|Default|SetMaterial (Rendering|Material|GetMaterial (Variables|Default|GetObjectBase) 0)))

(event Collision|EventActorBeginOverlap
  (params (OtherActor :type Actor%20Object%20Reference)))

(event EventTick
  (params (DeltaSeconds :type Float%20%28single-precision%29))
  (bind _objecttodisplay (Variables|Default|GetObjectToDisplay))
  (if (Variables|Default|GetPlayerIsOverlapping)
    (bind _asthird_person_character (Utilities|Casting|CastToThirdPersonCharacter (Game|Player|GetPlayerPawn 0)))
    (if (== (Variables|/Game/ThirdPersonBP/Blueprints/ThirdPersonCharacter.ThirdPersonCharacter_C|GetObjectType _asthird_person_character) (Variables|Default|GetObjectTypeRequirement))
      (Variables|/Game/ThirdPersonBP/Blueprints/ThirdPersonCharacter.ThirdPersonCharacter_C|SetTextToDisplay _asthird_person_character (Variables|Default|GetMyText))
      (if (Variables|/Game/ThirdPersonBP/Blueprints/ThirdPersonCharacter.ThirdPersonCharacter_C|GetClicking _asthird_person_character)
        (if (not (Variables|Default|GetObjetPut))
          (Variables|/Game/ThirdPersonBP/Blueprints/ThirdPersonCharacter.ThirdPersonCharacter_C|SetTextToDisplay _asthird_person_character "")
          (Variables|Default|SetObjetPut true)
          (Rendering|SetVisibility _objecttodisplay true false)
          (Collision|SetCollisionEnabled _objecttodisplay "QueryAndPhysics")
          (Rendering|Material|SetMaterial (Variables|Default|GetObjectBase) 0 "/Game/Assets/Meshes/Material_011.Material_011")
          (Variables|/Game/ThirdPersonBP/Blueprints/ThirdPersonCharacter.ThirdPersonCharacter_C|SetObjectType _asthird_person_character 0)
          (bind _rotz (Timeline|DoAnim Play)
            (:Update
              (Transformation|SetRelativeRotation (Variables|Default|GetDoorRoot) (Math|Rotator|MakeRotator 0.0 0.0 _rotz) false false))))))))

(fn ConstructionScript)

(fn Animation
  (params (RotZ :type Float%20%28single-precision%29)))